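; BP_GameEndAnimation is a trigger actor that plays the game's ending when the player enters its box.
; On overlap it toggles the player's hidden state and reveals a paper flipbook that starts hidden at BeginPlay.
; After short delays it adds the game end popup widget to the viewport, then opens the credits level.
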(event OnComponentBeginOverlap(Box)
  (params (OverlappedComponent :type Primitive%20Component%20Object%20Reference) (OtherActor :type Actor%20Object%20Reference) (OtherComp :type Primitive%20Component%20Object%20Reference) (OtherBodyIndex :type Integer) (bFromSweep :type Boolean) (SweepResult :type Hit%20Result%20Structure%20%28by%20ref%29))
  (bind _asbp_player (Utilities|Casting|CastToBP_Player OtherActor))
  (Default|ToggleHide _asbp_player)
  (Development|SetHiddeninGame (Variables|Default|GetPaperFlipbook) false false)
  (Utilities|FlowControl|Delay 1.5)
  (bind _returnvalue (UserInterface|CreateWidget "/Game/Levels/Programmers/Marwan/Widgets/GamePopups/W_GameEndPopup.W_GameEndPopup_C"))
  (UserInterface|Viewport|AddtoViewport _returnvalue 0)
  (Utilities|FlowControl|Delay 3.0)
  (Game|OpenLevel(byName) "M_Credits"))

(event EventBeginPlay
  (Development|SetHiddeninGame (Variables|Default|GetPaperFlipbook) true false))

(event Collision|EventActorBeginOverlap
  (params (OtherActor :type Actor%20Object%20Reference)))

(event EventTick
  (params (DeltaSeconds :type Float%20%28single-precision%29)))

(fn ConstructionScript)