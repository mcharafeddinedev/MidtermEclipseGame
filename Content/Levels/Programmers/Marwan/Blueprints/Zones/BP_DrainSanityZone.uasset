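; BP_DrainSanityZone is a zone Blueprint that lowers the player's sanity.
; DrainSanity subtracts DrainRate from the Sanity of PlayerREF and clamps the result between zero and MaxSanity.
; The event graph is empty, so nothing here calls the function or sets the player reference.
; The drain is a fixed step per call, as the delta-time multiply is left unconnected.
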(event EventBeginPlay)

(event Collision|EventActorBeginOverlap
  (params (OtherActor :type Actor%20Object%20Reference)))

(event EventTick
  (params (DeltaSeconds :type Float%20%28single-precision%29)))

(fn ConstructionScript)

(fn DrainSanity
  (Variables|/Game/Levels/Programmers/Justin/PrototypeBlueprints/BP_Player.BP_Player_C|SetSanity (Variables|Default|GetPlayerREF) (Math|Float|Clamp(Float) (- (Variables|/Game/Levels/Programmers/Justin/PrototypeBlueprints/BP_Player.BP_Player_C|GetSanity (Variables|Default|GetPlayerREF)) (Variables|Default|GetDrainRate)) 0.0 (Variables|/Game/Levels/Programmers/Justin/PrototypeBlueprints/BP_Player.BP_Player_C|GetMaxSanity (Variables|Default|GetPlayerREF)))))