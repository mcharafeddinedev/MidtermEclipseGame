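; BP_Paint is a prop that briefly reveals a hidden bloody-paint flipbook when the player enters its box trigger.
; On BP_Player overlap it plays the Hmmm sound, adds a W_ThatsOdd popup and shows the flipbook for one second before hiding it.
; Ending any overlap removes the popup, without checking the actor.
; The DoOnce sits at the end of the chain, so the effect repeats on re-entry.
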(event OnComponentBeginOverlap(Box)
  (params (OverlappedComponent :type Primitive%20Component%20Object%20Reference) (OtherActor :type Actor%20Object%20Reference) (OtherComp :type Primitive%20Component%20Object%20Reference) (OtherBodyIndex :type Integer) (bFromSweep :type Boolean) (SweepResult :type Hit%20Result%20Structure%20%28by%20ref%29))
  (Utilities|Casting|CastToBP_Player OtherActor)
  (Audio|PlaySound2D "/Game/Levels/Programmers/Marwan/MySFX/hmmm.hmmm" 1.0 1.0 0.0 0 0)
  ;[1 1 1] Popup Widget
  (bind _returnvalue (UserInterface|CreateWidget "/Game/Levels/Programmers/Marwan/Widgets/GamePopups/W_ThatsOdd.W_ThatsOdd_C"))
  (UserInterface|Viewport|AddtoViewport _returnvalue 0)
  ;[1 1 1] Show and then Hide again BloodyPaint BP
  (Development|SetHiddeninGame (Variables|Default|GetPaperFlipbook) false false)
  (Utilities|FlowControl|Delay 1.0)
  (Development|SetHiddeninGame (Variables|Default|GetPaperFlipbook) true false)
  (Utilities|FlowControl|DoOnce false))

(event OnComponentEndOverlap(Box)
  (params (OverlappedComponent :type Primitive%20Component%20Object%20Reference) (OtherActor :type Actor%20Object%20Reference) (OtherComp :type Primitive%20Component%20Object%20Reference) (OtherBodyIndex :type Integer))
  ;[1 1 1] Popup Widget
  (Widget|RemovefromParent (stale OnComponentBeginOverlap(Box) _returnvalue)))

(event EventBeginPlay
  ;[1 1 1] Set flipbook to hidden on Begin
  (Development|SetHiddeninGame (Variables|Default|GetPaperFlipbook) true false))

(event EventTick
  (params (DeltaSeconds :type Float%20%28single-precision%29)))

(fn ConstructionScript)