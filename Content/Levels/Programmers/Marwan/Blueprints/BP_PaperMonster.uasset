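; BP_PaperMonster is a Paper2D monster character that walks horizontally and reacts when BP_Player enters its sensing radius.
; Each tick it picks the idle or walk flipbook from velocity and turns the controller's yaw to face travel along X.
; The sensing overlap stores the player and adds a single movement input from the player's world X, not the relative direction.
; It retains a Move Right input handler and disconnected chase and animation logic.
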(event OnComponentBeginOverlap(SensingRadiusCollision)
  (params (OverlappedComponent :type Primitive%20Component%20Object%20Reference) (OtherActor :type Actor%20Object%20Reference) (OtherComp :type Primitive%20Component%20Object%20Reference) (OtherBodyIndex :type Integer) (bFromSweep :type Boolean) (SweepResult :type Hit%20Result%20Structure%20%28by%20ref%29))
  (bind _asbp_player (Utilities|Casting|CastToBP_Player OtherActor))
  (Variables|Default|SetPlayerREF _asbp_player)
  (Variables|Default|SetisMoving? true)
  (Class|PawnMovementComponent|AddInputVector (Variables|Character|GetCharacterMovement) (Math|Vector|MakeVector (Math|Conversions|ToFloat(Integer) (Utilities|String|ToString(Integer) (Utilities|Struct|MakeVector3f (.x (Transformation|GetActorLocation (Variables|Default|GetPlayerREF))) 0.0 0.0))) 0.0 0.0) false))

(event Custom|UpdateControlRotation
  ;[1 1 1] Lets you face left and right
  (Utilities|IsValid (Pawn|GetController)
    (:Is%20Valid
      (Math|Float|CompareFloat (.X (Math|Vector|BreakVector (Variables|/Script/Engine.MovementComponent|GetVelocity (Variables|Character|GetCharacterMovement)))) 0.0
        (:>
          (Pawn|SetControlRotation (Pawn|GetController) (Math|Rotator|MakeRotator 0.0 0.0 0.0)))
        (:<
          (Pawn|SetControlRotation (Pawn|GetController) (Math|Rotator|MakeRotator 0.0 0.0 1.8e+02)))))))

(event Custom|AnimationUpdate
  ;[1 1 1] Switches between idle and walking animations
  (Sprite|SetFlipbook (Variables|Default|GetSprite) (select (> (Math|Vector|VectorLength (Variables|/Script/Engine.MovementComponent|GetVelocity (Variables|Character|GetCharacterMovement))) 0.0) "/Game/Levels/Programmers/Marwan/Flipbooks/FB_MonsterWalk.FB_MonsterWalk" "/Game/Levels/Programmers/Marwan/Flipbooks/FB_MonsterIdle.FB_MonsterIdle")))

(event EventBeginPlay)

(event Collision|EventActorBeginOverlap
  (params (OtherActor :type Actor%20Object%20Reference)))

(event EventTick
  (params (DeltaSeconds :type Float%20%28single-precision%29))
  (CallFunction|AnimationUpdate)
  (CallFunction|UpdateControlRotation))

(event Input|AxisEvents|InputAxisMoveRight
  (params (AxisValue :type Float%20%28single-precision%29))
  ;[1 1 1] Moves you left to right
  (Pawn|Input|AddMovementInput "1.000000,0.000000,0.000000" AxisValue false))

(fn ConstructionScript)