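; Prototype 2D side-scrolling player character that walks, sprints, hides, changes levels through doors, collects orbs and reads notebooks.
; Movement input drives flipbook choice and left/right facing.
; Per-feature collision overlaps open and close Gates on Interact, triggering hiding, level loads, orb tallying or toggled notebook widgets.
; Pause shows a menu only while held and passes false to SetGamePaused; the three-orb goal check is unwired.
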(event OnComponentBeginOverlap(KeyItemCollision)
  (params (OverlappedComponent :type Primitive%20Component%20Object%20Reference) (OtherActor :type Actor%20Object%20Reference) (OtherComp :type Primitive%20Component%20Object%20Reference) (OtherBodyIndex :type Integer) (bFromSweep :type Boolean) (SweepResult :type Hit%20Result%20Structure%20%28by%20ref%29))
  ;[1 1 1] Allows you to grab the orbs and have them be added to the tally/ goal of collecting 3 orbs
  (bind _asbp_interactive_item (Utilities|Casting|CastToBP_InteractiveItem OtherActor))
  (Input|EnableInput 0)
  (Utilities|FlowControl|Gate true) ; enters at Open
)

(event OnComponentEndOverlap(KeyItemCollision)
  (params (OverlappedComponent :type Primitive%20Component%20Object%20Reference) (OtherActor :type Actor%20Object%20Reference) (OtherComp :type Primitive%20Component%20Object%20Reference) (OtherBodyIndex :type Integer))
  ;[1 1 1] Allows you to grab the orbs and have them be added to the tally/ goal of collecting 3 orbs
  (Utilities|Casting|CastToBP_InteractiveItem OtherActor)
  (Input|EnableInput 0)
  (Utilities|FlowControl|Gate true) ; enters at Close
)

(event OnComponentBeginOverlap(ExitDoorCollision)
  (params (OverlappedComponent :type Primitive%20Component%20Object%20Reference) (OtherActor :type Actor%20Object%20Reference) (OtherComp :type Primitive%20Component%20Object%20Reference) (OtherBodyIndex :type Integer) (bFromSweep :type Boolean) (SweepResult :type Hit%20Result%20Structure%20%28by%20ref%29))
  ;[1 1 1] Allows you to go from the hallway to the room and back (PROTOTYPE MUST FIX)
  (Utilities|Casting|CastToBP_ExitDoor OtherActor)
  (Input|EnableInput 0)
  (Utilities|FlowControl|Gate true) ; enters at Open
)

(event OnComponentEndOverlap(ExitDoorCollision)
  (params (OverlappedComponent :type Primitive%20Component%20Object%20Reference) (OtherActor :type Actor%20Object%20Reference) (OtherComp :type Primitive%20Component%20Object%20Reference) (OtherBodyIndex :type Integer))
  ;[1 1 1] Allows you to go from the hallway to the room and back (PROTOTYPE MUST FIX)
  (Utilities|Casting|CastToBP_ExitDoor OtherActor)
  (Input|EnableInput 0)
  (Utilities|FlowControl|Gate true) ; enters at Close
)

(event OnComponentBeginOverlap(NotebookCollision2)
  (params (OverlappedComponent :type Primitive%20Component%20Object%20Reference) (OtherActor :type Actor%20Object%20Reference) (OtherComp :type Primitive%20Component%20Object%20Reference) (OtherBodyIndex :type Integer) (bFromSweep :type Boolean) (SweepResult :type Hit%20Result%20Structure%20%28by%20ref%29))
  ;[1 1 1] Allows you to bring up specific widget for notebook and have it be deleted when you walk away
  (Utilities|Casting|CastToBP_Notebook2 OtherActor)
  (Input|EnableInput 0)
  (Utilities|FlowControl|Gate true) ; enters at Open
)

(event OnComponentEndOverlap(NotebookCollision2)
  (params (OverlappedComponent :type Primitive%20Component%20Object%20Reference) (OtherActor :type Actor%20Object%20Reference) (OtherComp :type Primitive%20Component%20Object%20Reference) (OtherBodyIndex :type Integer))
  ;[1 1 1] Allows you to bring up specific widget for notebook and have it be deleted when you walk away
  (Utilities|Casting|CastToBP_Notebook2 OtherActor)
  (Input|EnableInput 0)
  (UserInterface|CreateWidget "/Game/Levels/Programmers/Justin/PrototypeBlueprints/NotebookBP/NotebookWidgets/W_Notebook2.W_Notebook2_C")
  (Widget|RemovefromParent (Variables|Default|GetWidgetRef2))
  (Utilities|FlowControl|Gate true) ; enters at Close
)

(event OnComponentBeginOverlap(NotebookCollision3)
  (params (OverlappedComponent :type Primitive%20Component%20Object%20Reference) (OtherActor :type Actor%20Object%20Reference) (OtherComp :type Primitive%20Component%20Object%20Reference) (OtherBodyIndex :type Integer) (bFromSweep :type Boolean) (SweepResult :type Hit%20Result%20Structure%20%28by%20ref%29))
  ;[1 1 1] Allows you to bring up specific widget for notebook and have it be deleted when you walk away
  (Utilities|Casting|CastToBP_Notebook3 OtherActor)
  (Input|EnableInput 0)
  (Utilities|FlowControl|Gate true) ; enters at Open
)

(event OnComponentEndOverlap(NotebookCollision3)
  (params (OverlappedComponent :type Primitive%20Component%20Object%20Reference) (OtherActor :type Actor%20Object%20Reference) (OtherComp :type Primitive%20Component%20Object%20Reference) (OtherBodyIndex :type Integer))
  ;[1 1 1] Allows you to bring up specific widget for notebook and have it be deleted when you walk away
  (Utilities|Casting|CastToBP_Notebook3 OtherActor)
  (Input|EnableInput 0)
  (UserInterface|CreateWidget "/Game/Levels/Programmers/Justin/PrototypeBlueprints/NotebookBP/NotebookWidgets/W_Notebook3.W_Notebook3_C")
  (Widget|RemovefromParent (Variables|Default|GetWidgetRef3))
  (Utilities|FlowControl|Gate true) ; enters at Close
)

(event OnComponentBeginOverlap(HidingCollision)
  (params (OverlappedComponent :type Primitive%20Component%20Object%20Reference) (OtherActor :type Actor%20Object%20Reference) (OtherComp :type Primitive%20Component%20Object%20Reference) (OtherBodyIndex :type Integer) (bFromSweep :type Boolean) (SweepResult :type Hit%20Result%20Structure%20%28by%20ref%29))
  ;[1 1 1] Allows to hide/unhide
  (Utilities|Casting|CastToBP_HidingPlace OtherActor)
  (Input|EnableInput 0)
  (Utilities|FlowControl|Gate true) ; enters at Open
)

(event OnComponentEndOverlap(HidingCollision)
  (params (OverlappedComponent :type Primitive%20Component%20Object%20Reference) (OtherActor :type Actor%20Object%20Reference) (OtherComp :type Primitive%20Component%20Object%20Reference) (OtherBodyIndex :type Integer))
  ;[1 1 1] Allows to hide/unhide
  (Utilities|Casting|CastToBP_HidingPlace OtherActor)
  (Input|EnableInput 0)
  (Utilities|FlowControl|Gate true) ; enters at Close
)

(event OnComponentBeginOverlap(NotebookCollision)
  (params (OverlappedComponent :type Primitive%20Component%20Object%20Reference) (OtherActor :type Actor%20Object%20Reference) (OtherComp :type Primitive%20Component%20Object%20Reference) (OtherBodyIndex :type Integer) (bFromSweep :type Boolean) (SweepResult :type Hit%20Result%20Structure%20%28by%20ref%29))
  ;[1 1 1] Allows you to bring up specific widget for notebook and have it be deleted when you walk away
  (Utilities|Casting|CastToBP_Notebook OtherActor)
  (Input|EnableInput 0)
  (Utilities|FlowControl|Gate true) ; enters at Open
)

(event OnComponentEndOverlap(NotebookCollision)
  (params (OverlappedComponent :type Primitive%20Component%20Object%20Reference) (OtherActor :type Actor%20Object%20Reference) (OtherComp :type Primitive%20Component%20Object%20Reference) (OtherBodyIndex :type Integer))
  ;[1 1 1] Allows you to bring up specific widget for notebook and have it be deleted when you walk away
  (Utilities|Casting|CastToBP_Notebook OtherActor)
  (Input|EnableInput 0)
  (UserInterface|CreateWidget "/Game/Levels/Programmers/Justin/PrototypeBlueprints/NotebookBP/NotebookWidgets/W_Notebook.W_Notebook_C")
  (Widget|RemovefromParent (Variables|Default|GetWidgetRef))
  (Utilities|FlowControl|Gate true) ; enters at Close
)

(event OnComponentBeginOverlap(DoorCollision)
  (params (OverlappedComponent :type Primitive%20Component%20Object%20Reference) (OtherActor :type Actor%20Object%20Reference) (OtherComp :type Primitive%20Component%20Object%20Reference) (OtherBodyIndex :type Integer) (bFromSweep :type Boolean) (SweepResult :type Hit%20Result%20Structure%20%28by%20ref%29))
  ;[1 1 1] Allows you to go from the hallway to the room and back (PROTOTYPE MUST FIX)
  (Utilities|Casting|CastToBP_Door OtherActor)
  (Input|EnableInput 0)
  (Utilities|FlowControl|Gate true) ; enters at Open
)

(event OnComponentEndOverlap(DoorCollision)
  (params (OverlappedComponent :type Primitive%20Component%20Object%20Reference) (OtherActor :type Actor%20Object%20Reference) (OtherComp :type Primitive%20Component%20Object%20Reference) (OtherBodyIndex :type Integer))
  ;[1 1 1] Allows you to go from the hallway to the room and back (PROTOTYPE MUST FIX)
  (Utilities|Casting|CastToBP_Door OtherActor)
  (Input|EnableInput 0)
  (Utilities|FlowControl|Gate true) ; enters at Close
)

(event Custom|UpdateAnimation
  ;[1 1 1] Switches between idle and walking animations
  (if (Variables|Default|GetWalking?)
    (if (Variables|Default|GetIsSprinting?)
      (Sprite|SetFlipbook (Variables|Default|GetSprite) "/Game/Artists/Laura/ANimations/Sprint/Broody_Sprint_Spriteshet1.Broody_Sprint_Spriteshet1")
      (else
        (Sprite|SetFlipbook (Variables|Default|GetSprite) "/Game/Artists/Laura/ANimations/Walking/Broody_Walking_Spriteshet1.Broody_Walking_Spriteshet1")))
    (else
      (Sprite|SetFlipbook (Variables|Default|GetSprite) "/Game/Artists/Laura/ANimations/Idle/Broody_Idle_1_Sprite_sheet1.Broody_Idle_1_Sprite_sheet1"))))

(event Custom|UpdateControlRotation
  ;[1 1 1] Lets you face left and right
  (Utilities|IsValid (Pawn|GetController)
    (:Is%20Valid
      (Math|Float|CompareFloat (.X (Math|Vector|BreakVector (Variables|/Script/Engine.MovementComponent|GetVelocity (Variables|Character|GetCharacterMovement)))) 0.0
        (:>
          (Pawn|SetControlRotation (Pawn|GetController) (Math|Rotator|MakeRotator 0.0 0.0 0.0)))
        (:<
          (Pawn|SetControlRotation (Pawn|GetController) (Math|Rotator|MakeRotator 0.0 0.0 1.8e+02)))))))

(event EventTick
  (params (DeltaSeconds :type Float%20%28single-precision%29))
  ;[1 1 1] Moves you left to right
  (Utilities|FlowControl|Sequence
    (:then_0
      (if (> (Math|Vector|VectorLength (Variables|/Script/Engine.MovementComponent|GetVelocity (Variables|Character|GetCharacterMovement))) 1e+01)
        (Variables|Default|SetWalking? true)
        (else
          (Variables|Default|SetWalking? false))))))

(event Input|ActionEvents|InputActionSprint
  (params (Key :type Key%20Structure :default "None"))
  (bind _charactermovement (Variables|Character|GetCharacterMovement))
  ;[1 1 1] Allows you to sprint(Need to add sprint animation)
  (:Pressed
    (Variables|/Script/Engine.CharacterMovementComponent|SetMaxWalkSpeed _charactermovement 2e+02)
    (Variables|Default|SetIsSprinting? true))
  (:Released
    (Variables|/Script/Engine.CharacterMovementComponent|SetMaxWalkSpeed _charactermovement 1e+02)
    (Variables|Default|SetIsSprinting? false)))

(event Input|ActionEvents|InputActionInteract
  (params (Key :type Key%20Structure :default "None"))
  ;[1 1 1] Allows you to go from the hallway to the room and back (PROTOTYPE MUST FIX)
  (:Pressed
    (Utilities|FlowControl|Gate true
      (:Exit
        (Game|OpenLevel(byObjectReference) "/Game/Levels/Programmers/Justin/PrototypeLevels/Prototype.Prototype")))))

(event Input|ActionEvents|InputActionInteract
  (params (Key :type Key%20Structure :default "None"))
  ;[1 1 1] Allows to hide/unhide
  (:Pressed
    (Utilities|FlowControl|Gate true :!label _label
      (:Exit
        (CallFunction|ToggleHide)
        (Utilities|FlowControl|Delay 0.2)
        (Input|EnableInput 0)
        (goto _label Open)))))

(event Input|ActionEvents|InputActionInteract
  (params (Key :type Key%20Structure :default "None"))
  ;[1 1 1] Allows you to go from the hallway to the room and back (PROTOTYPE MUST FIX)
  (:Pressed
    (Utilities|FlowControl|Gate true
      (:Exit
        (Game|OpenLevel(byObjectReference) "/Game/Levels/Programmers/Justin/PrototypeLevels/PrototypeRoom.PrototypeRoom")))))

(event Input|ActionEvents|InputActionInteract
  (params (Key :type Key%20Structure :default "None"))
  ;[1 1 1] Allows you to grab the orbs and have them be added to the tally/ goal of collecting 3 orbs
  (:Pressed
    (Utilities|FlowControl|Gate true
      (:Exit
        (Variables|Default|SetOrbNumber (+ (Variables|Default|GetOrbNumber) 1.0))
        (Actor|DestroyActor (stale OnComponentBeginOverlap(KeyItemCollision) _asbp_interactive_item))))))

(event Input|ActionEvents|InputActionInteract
  (params (Key :type Key%20Structure :default "None"))
  ;[1 1 1] Allows you to bring up specific widget for notebook and have it be deleted when you walk away
  (:Pressed
    (Utilities|FlowControl|Gate true
      (:Exit
        (Utilities|FlowControl|FlipFlop
          (:A
            (bind _returnvalue (UserInterface|CreateWidget "/Game/Levels/Programmers/Justin/PrototypeBlueprints/NotebookBP/NotebookWidgets/W_Notebook3.W_Notebook3_C"))
            (bind _output_get (Variables|Default|SetWidgetRef3 _returnvalue))
            (UserInterface|Viewport|AddtoViewport _output_get 0))
          (:B
            (UserInterface|CreateWidget "/Game/Levels/Programmers/Justin/PrototypeBlueprints/NotebookBP/NotebookWidgets/W_Notebook3.W_Notebook3_C")
            (Widget|RemovefromParent (Variables|Default|GetWidgetRef3))))))))

(event Input|ActionEvents|InputActionPause
  (params (Key :type Key%20Structure :default "None"))
  ;[1 0.6131 0] MC -- "Pause" Menu Functionality
  (:Pressed
    (Variables|Default|SetPaused? true)
    (Game|SetGamePaused false)
    (bind _returnvalue (UserInterface|CreateWidget "/Game/Levels/Programmers/Marwan/Widgets/W_PauseMenu.W_PauseMenu_C"))
    (UserInterface|Viewport|AddtoViewport _returnvalue 0)
    (bind _returnvalue_2 (Class|InputDeviceLibrary|GetPlayerControllerfromInputDevice))
    (Variables|/Script/Engine.PlayerController|SetbShowMouseCursor _returnvalue_2 true))
  (:Released
    (Variables|Default|SetPaused? false)
    (bind _returnvalue_3 (Class|InputDeviceLibrary|GetPlayerControllerfromInputDevice))
    (Variables|/Script/Engine.PlayerController|SetbShowMouseCursor _returnvalue_3 false)
    (Widget|RemovefromParent _returnvalue)))

(event Input|ActionEvents|InputActionInteract
  (params (Key :type Key%20Structure :default "None"))
  ;[1 1 1] Allows you to bring up specific widget for notebook and have it be deleted when you walk away
  (:Pressed
    (Utilities|FlowControl|Gate true
      (:Exit
        (Utilities|FlowControl|FlipFlop
          (:A
            (bind _returnvalue (UserInterface|CreateWidget "/Game/Levels/Programmers/Justin/PrototypeBlueprints/NotebookBP/NotebookWidgets/W_Notebook.W_Notebook_C"))
            (bind _output_get (Variables|Default|SetWidgetRef _returnvalue))
            (UserInterface|Viewport|AddtoViewport _output_get 0))
          (:B
            (UserInterface|CreateWidget "/Game/Levels/Programmers/Justin/PrototypeBlueprints/NotebookBP/NotebookWidgets/W_Notebook.W_Notebook_C")
            (Widget|RemovefromParent (Variables|Default|GetWidgetRef))))))))

(event Input|ActionEvents|InputActionInteract
  (params (Key :type Key%20Structure :default "None"))
  ;[1 1 1] Allows you to bring up specific widget for notebook and have it be deleted when you walk away
  (:Pressed
    (Utilities|FlowControl|Gate true
      (:Exit
        (Utilities|FlowControl|FlipFlop
          (:A
            (bind _returnvalue (UserInterface|CreateWidget "/Game/Levels/Programmers/Justin/PrototypeBlueprints/NotebookBP/NotebookWidgets/W_Notebook2.W_Notebook2_C"))
            (bind _output_get (Variables|Default|SetWidgetRef2 _returnvalue))
            (UserInterface|Viewport|AddtoViewport _output_get 0))
          (:B
            (UserInterface|CreateWidget "/Game/Levels/Programmers/Justin/PrototypeBlueprints/NotebookBP/NotebookWidgets/W_Notebook2.W_Notebook2_C")
            (Widget|RemovefromParent (Variables|Default|GetWidgetRef2))))))))

(event Input|AxisEvents|InputAxisMoveRight
  (params (AxisValue :type Float%20%28single-precision%29))
  ;[1 1 1] Moves you left to right
  (CallFunction|UpdateAnimation)
  (CallFunction|UpdateControlRotation)
  (Pawn|Input|AddMovementInput "1.000000,0.000000,0.000000" AxisValue false))

(fn ConstructionScript)

(fn ToggleHide
  (if (Variables|Default|GetIsHiding?)
    (Variables|Default|SetIsHiding? false)
    (Rendering|SetActorHiddenInGame true)
    (Collision|SetActorEnableCollision false)
    (else
      (Variables|Default|SetIsHiding? true)
      (Rendering|SetActorHiddenInGame false)
      (Collision|SetActorEnableCollision true))))